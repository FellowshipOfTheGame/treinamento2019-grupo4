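; Door actor that swings open and loads CityLevel when the player character enters its trigger.
; Trigger begin and end overlaps switch a target rotator between open and closed.
; Tick continuously eases the Scene component's relative rotation toward that target with RInterpTo.
; The level opens immediately on overlap, without waiting for the swing to finish.
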(event OnComponentBeginOverlap(Trigger)
  (params (OverlappedComponent :type Primitive%20Component%20Object%20Reference) (OtherActor :type Actor%20Object%20Reference) (OtherComp :type Primitive%20Component%20Object%20Reference) (OtherBodyIndex :type Integer) (bFromSweep :type Boolean) (SweepResult :type Hit%20Result%20Structure%20%28by%20ref%29))
  (if (== OtherActor (Game|GetPlayerCharacter 0))
    (Variables|Default|SetRotator "0,90.000000, 0")
    (Game|OpenLevel(byName) "CityLevel")))

(event OnComponentEndOverlap(Trigger)
  (params (OverlappedComponent :type Primitive%20Component%20Object%20Reference) (OtherActor :type Actor%20Object%20Reference) (OtherComp :type Primitive%20Component%20Object%20Reference) (OtherBodyIndex :type Integer))
  (if (== (Game|GetPlayerCharacter 0) OtherActor)
    (Variables|Default|SetRotator "0,0.000000, 0")))

(event EventBeginPlay
  (Variables|Default|SetRotator "0,0.000000, 0"))

(event Collision|EventActorBeginOverlap
  (params (OtherActor :type Actor%20Object%20Reference)))

(event EventTick
  (params (DeltaSeconds :type Float%20%28single-precision%29))
  (bind _scene (Variables|Default|GetScene))
  (Transformation|SetRelativeRotation _scene (Math|Interpolation|RInterpTo (Variables|/Script/Engine.SceneComponent|GetRelativeRotation _scene) (Variables|Default|GetRotator) DeltaSeconds 1e+01) false false))

(fn ConstructionScript)